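; Player character Blueprint that adds speed-based camera head bob and footstep sounds.
; The CameraAnimation event plays the HeadWobble timeline, whose alpha drives the camera's relative Z offset.
; Horizontal velocity, mapped against max walk speed, scales both the bob height and the timeline's play rate.
; A timeline event track plays indoor or outdoor footstep cues based on IsOutdoor while moving on the ground, keeping steps synced to the bob.
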(event EventCameraAnimation
  (bind _charactermovement (Variables|Character|GetCharacterMovement))
  (bind _velocity (Variables|/Script/Engine.MovementComponent|GetVelocity _charactermovement))
  (bind _maxwalkspeed (Variables|/Script/Engine.CharacterMovementComponent|GetMaxWalkSpeed _charactermovement))
  (bind _returnvalue (Math|Vector|VectorLengthXY _velocity))
  (bind _returnvalue_2 (Math|Float|MapRangeClamped _returnvalue 0.0 _maxwalkspeed 0.0 1.1))
  ;[1 1 1] Head Wobble
  (bind _alpha (Timeline|HeadWobble Play)
    (:Update
      (Transformation|SetRelativeLocation (Variables|Default|GetCamera) (Math|Vector|MakeVector 0.0 0.0 (* _alpha (Variables|Default|GetHeadMovementIntensity) _returnvalue_2)) false false)
      (Variables|Default|SetHeadMovementIntensity _returnvalue_2)
      (Components|Timeline|SetPlayRate (Variables|Default|GetHeadWobble) (Variables|Default|GetHeadMovementIntensity)))
    (:Event
      (if (and (AI|Components|NavMovement|IsMovingonGround _charactermovement) (> _returnvalue 5e+01))
        (if (Variables|Default|GetIsOutdoor)
          (Audio|PlaySoundatLocation "/Game/PlanetRetrofit/Sounds/Player/Footsteps/Outdoor/Cue_OutdoorFootsteps.Cue_OutdoorFootsteps" (Transformation|GetActorLocation) "0, 0, 0" 1.0 1.0 0.0 0 0 0 0)
          (else
            (Audio|PlaySoundatLocation "/Game/PlanetRetrofit/Sounds/Player/Footsteps/Indoor/Cue_IndoorFootsteps.Cue_IndoorFootsteps" (Transformation|GetActorLocation) "0, 0, 0" 1.0 1.0 0.0 0 0 0 0)))))))

(fn ConstructionScript)